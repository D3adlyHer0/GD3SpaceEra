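; Bp_jug is a perk pickup that sells the player a one-time health boost in exchange for Score.
; Overlapping its box with a "player"-tagged character sets a range flag and shows the UI_bonushealth prompt, which is removed on end overlap.
; The bonushealth event uses that flag and a DoOnce gate to deduct score and add health, resetting only when the player is away or short on score.
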(event `self.Box.OnComponentBeginOverlap`
  (params (OverlappedComponent :type "PrimitiveComponent Object Reference") (OtherActor :type "Actor Object Reference") (OtherComp :type "PrimitiveComponent Object Reference") (OtherBodyIndex :type Integer) (bFromSweep :type Boolean) (SweepResult :type "HitResult Structure (by ref)"))
  (if (`self.ActorHasTag` OtherActor "player")
    (set `self.playertrue?` true)
    (cast `/Game/ThirdPerson/Blueprints/BP_ThirdPersonCharacterSynty` OtherActor)
    (bind _returnvalue (`|CreateWidget` "/Game/Ryan_design/ui/UI_bonushealth.UI_bonushealth_C" (`GameplayStatics.GetPlayerController` 0)))
    (`UserWidget.AddToPlayerScreen` _returnvalue 0)))

(event `bonus health`
  (`/Engine/EditorBlueprintResources/StandardMacros.DoOnce` false :!label _label
    (:`Completed`
      (if (`self.playertrue?`)
        (bind _asbp_third_person_character_synty (cast `/Game/ThirdPerson/Blueprints/BP_ThirdPersonCharacterSynty` (stale `self.Box.OnComponentBeginOverlap` OtherActor)))
        (bind _score (`/Game/ThirdPerson/Blueprints/BP_ThirdPersonCharacterSynty.score` _asbp_third_person_character_synty))
        (if (>= _score 950.0)
          (set `/Game/ThirdPerson/Blueprints/BP_ThirdPersonCharacterSynty.score` (- _score 950.0) _asbp_third_person_character_synty)
          (set `/Game/ThirdPerson/Blueprints/BP_ThirdPersonCharacterSynty.health` (+ (`/Game/ThirdPerson/Blueprints/BP_ThirdPersonCharacterSynty.health` _asbp_third_person_character_synty) 150.0) _asbp_third_person_character_synty)
          (`Widget.RemoveFromParent` (stale `self.Box.OnComponentBeginOverlap` _returnvalue))
          (else
            (`KismetSystemLibrary.PrintString` "come back later")
            (goto _label :!via `Reset`)))
        (else
          (goto _label :!via `Reset`))))))

(event `self.Box.OnComponentEndOverlap`
  (params (OverlappedComponent :type "PrimitiveComponent Object Reference") (OtherActor :type "Actor Object Reference") (OtherComp :type "PrimitiveComponent Object Reference") (OtherBodyIndex :type Integer))
  (set `self.playertrue?` false)
  (`Widget.RemoveFromParent` (stale `self.Box.OnComponentBeginOverlap` _returnvalue)))

(fn `UserConstructionScript`)