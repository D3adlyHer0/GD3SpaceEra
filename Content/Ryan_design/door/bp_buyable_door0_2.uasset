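; Buyable door that the player purchases with score, destroying itself and activating matching spawners.
; Overlapping Buybox with a "player"-tagged actor sets Playertrue, which is never cleared in this graph.
; The opendoor event checks that flag, deducts a fixed Score cost from the player character, then calls DoorOpen on every Bp_spawn0 with the same ChannelID.
; A DoOnce guards the purchase and resets when the flag is unset or Score is too low.
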(event `self.buybox.OnComponentBeginOverlap`
  (params (OverlappedComponent :type "PrimitiveComponent Object Reference") (OtherActor :type "Actor Object Reference") (OtherComp :type "PrimitiveComponent Object Reference") (OtherBodyIndex :type Integer) (bFromSweep :type Boolean) (SweepResult :type "HitResult Structure (by ref)"))
  (if (`self.ActorHasTag` OtherActor "player")
    (set `self.playertrue?` true)))

(event `open door`
  (`/Engine/EditorBlueprintResources/StandardMacros.DoOnce` false :!label _label
    (:`Completed`
      (if (`self.playertrue?`)
        (bind _asbp_ryan_testier_shooting (cast `/Game/Ryan_design/ai_players/Bp_ryan_testier_shooting` (`GameplayStatics.GetPlayerCharacter` 0)))
        (if (>= (`/Game/Ryan_design/ai_players/Bp_ryan_testier_shooting.score` _asbp_ryan_testier_shooting) 850.0)
          (set `/Game/Ryan_design/ai_players/Bp_ryan_testier_shooting.score` (- (`/Game/Ryan_design/ai_players/Bp_ryan_testier_shooting.score` _asbp_ryan_testier_shooting) 850.0) _asbp_ryan_testier_shooting)
          (`self.K2_DestroyActor`)
          (bind _outactors (`GameplayStatics.GetAllActorsOfClass` "/Game/Ryan_design/spaners/bp_spawn0.bp_spawn0_C"))
          (for _array_element _outactors
            (if (== (`/Game/Ryan_design/spaners/bp_spawn0.channel ID ` _array_element) (`self.channel ID`))
              (`/Game/Ryan_design/spaners/bp_spawn0.door open` _array_element)))
          (else
            (`KismetSystemLibrary.PrintString` "come back later")
            (goto _label :!via `Reset`)))
        (else
          (goto _label :!via `Reset`))))))

(fn `UserConstructionScript`)