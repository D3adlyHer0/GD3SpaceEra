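; Purchasable door actor that a player can remove by spending 850 score, activating its linked spawners.
; Overlapping the Buybox flags the player as in range and shows a door prompt widget, which is removed on exit.
; The opendoor event, gated by a resettable DoOnce, checks range and score, deducts the cost, destroys the door and calls DoorOpen on Bp_spawn6 actors with a matching ChannelID.
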(event `self.buybox.OnComponentBeginOverlap`
  (params (OverlappedComponent :type "PrimitiveComponent Object Reference") (OtherActor :type "Actor Object Reference") (OtherComp :type "PrimitiveComponent Object Reference") (OtherBodyIndex :type Integer) (bFromSweep :type Boolean) (SweepResult :type "HitResult Structure (by ref)"))
  (if (`self.ActorHasTag` OtherActor "player")
    (set `self.playertrue?` true)
    (cast `/Game/ThirdPerson/Blueprints/BP_ThirdPersonCharacterSynty` OtherActor)
    (bind _returnvalue (`|CreateWidget` "/Game/Ryan_design/ui/UI_door_text.UI_door_text_C" (`GameplayStatics.GetPlayerController` 0)))
    (`UserWidget.AddToPlayerScreen` _returnvalue 0)))

(event `open door`
  (`/Engine/EditorBlueprintResources/StandardMacros.DoOnce` false :!label _label
    (:`Completed`
      (if (`self.playertrue?`)
        (bind _asbp_third_person_character_synty (cast `/Game/ThirdPerson/Blueprints/BP_ThirdPersonCharacterSynty` (stale `self.buybox.OnComponentBeginOverlap` OtherActor)))
        (bind _score (`/Game/ThirdPerson/Blueprints/BP_ThirdPersonCharacterSynty.score` _asbp_third_person_character_synty))
        (if (>= _score 850.0)
          (set `/Game/ThirdPerson/Blueprints/BP_ThirdPersonCharacterSynty.score` (- _score 850.0) _asbp_third_person_character_synty)
          (`Widget.RemoveFromParent` (stale `self.buybox.OnComponentBeginOverlap` _returnvalue))
          (`self.K2_DestroyActor`)
          (bind _outactors (`GameplayStatics.GetAllActorsOfClass` "/Game/Ryan_design/spaners/bp_spawn6.bp_spawn6_C"))
          (for _array_element _outactors
            (if (== (`/Game/Ryan_design/spaners/bp_spawn6.channel ID ` _array_element) (`self.channel ID`))
              (`/Game/Ryan_design/spaners/bp_spawn6.door open` _array_element)))
          (else
            (`KismetSystemLibrary.PrintString` "come back later")
            (goto _label :!via `Reset`)))
        (else
          (goto _label :!via `Reset`))))))

(event `self.buybox.OnComponentEndOverlap`
  (params (OverlappedComponent :type "PrimitiveComponent Object Reference") (OtherActor :type "Actor Object Reference") (OtherComp :type "PrimitiveComponent Object Reference") (OtherBodyIndex :type Integer))
  (set `self.playertrue?` false)
  (`Widget.RemoveFromParent` (stale `self.buybox.OnComponentBeginOverlap` _returnvalue)))

(fn `UserConstructionScript`)