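; Power switch actor that sells the game's victory: a player in range can spend 5000 Score to win.
; Its Box overlap tracks the tagged player and shows the UI_Power prompt.
; The poweron event, gated by a DoOnce that resets on insufficient Score, deducts the cost, disables movement and shows VictoryMeny with a cursor.
; A loop opening buyable doors by matching ChannelID is left unconnected.
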(event `self.Box.OnComponentBeginOverlap`
  (params (OverlappedComponent :type "PrimitiveComponent Object Reference") (OtherActor :type "Actor Object Reference") (OtherComp :type "PrimitiveComponent Object Reference") (OtherBodyIndex :type Integer) (bFromSweep :type Boolean) (SweepResult :type "HitResult Structure (by ref)"))
  (if (`self.ActorHasTag` OtherActor "player")
    (set `self.playertrue?` true)
    (cast `/Game/ThirdPerson/Blueprints/BP_ThirdPersonCharacterSynty` OtherActor)
    (bind _returnvalue (`|CreateWidget` "/Game/Ryan_design/ui/UI_Power.UI_Power_C" (`GameplayStatics.GetPlayerController` 0)))
    (`UserWidget.AddToPlayerScreen` _returnvalue 0)))

(event `self.Box.OnComponentEndOverlap`
  (params (OverlappedComponent :type "PrimitiveComponent Object Reference") (OtherActor :type "Actor Object Reference") (OtherComp :type "PrimitiveComponent Object Reference") (OtherBodyIndex :type Integer))
  (set `self.playertrue?` false)
  (`Widget.RemoveFromParent` (stale `self.Box.OnComponentBeginOverlap` _returnvalue)))

(event `power on`
  (`/Engine/EditorBlueprintResources/StandardMacros.DoOnce` false :!label _label
    (:`Completed`
      (if (`self.playertrue?`)
        (bind _asbp_third_person_character_synty (cast `/Game/ThirdPerson/Blueprints/BP_ThirdPersonCharacterSynty` (stale `self.Box.OnComponentBeginOverlap` OtherActor)))
        (bind _score (`/Game/ThirdPerson/Blueprints/BP_ThirdPersonCharacterSynty.score` _asbp_third_person_character_synty))
        (if (>= _score 5000.0)
          (set `/Game/ThirdPerson/Blueprints/BP_ThirdPersonCharacterSynty.score` (- _score 5000.0) _asbp_third_person_character_synty)
          (`Widget.RemoveFromParent` (stale `self.Box.OnComponentBeginOverlap` _returnvalue))
          (`CharacterMovementComponent.DisableMovement` (`Character.CharacterMovement` _asbp_third_person_character_synty))
          (bind _returnvalue (`|CreateWidget` "/Game/DylanStuff/VictoryMeny.VictoryMeny_C"))
          (`UserWidget.AddToViewport` _returnvalue 0)
          (set `PlayerController.bShowMouseCursor` true (`GameplayStatics.GetPlayerController` 0))
          (else
            (`KismetSystemLibrary.PrintString` "try later")
            (goto _label :!via `Reset`)))))))

(fn `UserConstructionScript`)