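; Test zombie AI enemy that chases the player and deals damage on contact.
; It repeatedly issues AI MoveTo toward the player character, restarting on success and printing a message on failure.
; Overlapping HitPlayerBox with a "Player"-tagged actor starts a delayed damage loop that has no end-overlap stop.
; Incoming damage lowers Health, destroys the zombie at zero and adds Score to Bp_ryan_testier_shooting on every hit.
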(event `self.ReceiveBeginPlay`
  (`self.movezombie`))

(event `movezombie`
  (`|AIMoveTo` self (0.0 0.0 0.0) (`GameplayStatics.GetPlayerCharacter` 0) :!label _label
    (:`OnSuccess`
      (`self.movezombie`)
      (`KismetSystemLibrary.Delay` 0.2)
      (goto _label))
    (:`OnFail`
      (`KismetSystemLibrary.PrintString` "you suck"))))

(event `self.ReceiveAnyDamage`
  (params (Damage :type "Float (single-precision)") (DamageType :type "DamageType Object Reference") (InstigatedBy :type "Controller Object Reference") (DamageCauser :type "Actor Object Reference"))
  ;[1 1 1] TakeDamage
  (`|ExecutionSequence`
    (:`then_0`
      (bind _output_get (set `self.Health` (- (`self.Health`) Damage)))
      (`KismetSystemLibrary.PrintString` (`KismetStringLibrary.Conv_DoubleToString` _output_get))
      (if (<= (`self.Health`) 0.0)
        (`self.K2_DestroyActor`)))
    (:`then_1`
      (bind _asbp_ryan_testier_shooting (cast `/Game/Ryan_design/ai_players/Bp_ryan_testier_shooting` (`GameplayStatics.GetPlayerCharacter` 0)))
      (set `/Game/Ryan_design/ai_players/Bp_ryan_testier_shooting.score` (+ (`/Game/Ryan_design/ai_players/Bp_ryan_testier_shooting.score` _asbp_ryan_testier_shooting) 20.0) _asbp_ryan_testier_shooting))))

(event `self.hit player box.OnComponentBeginOverlap`
  (params (OverlappedComponent :type "PrimitiveComponent Object Reference") (OtherActor :type "Actor Object Reference") (OtherComp :type "PrimitiveComponent Object Reference") (OtherBodyIndex :type Integer) (bFromSweep :type Boolean) (SweepResult :type "HitResult Structure (by ref)"))
  (if (`self.ActorHasTag` OtherActor "Player")
    (`GameplayStatics.ApplyDamage` OtherActor 10.0 null self :!label _label_2)
    (`KismetSystemLibrary.Delay` 1.5)
    (goto _label_2)))

(event `ResetAttack`)

(fn `UserConstructionScript`)