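; Test zombie AI pawn that chases the first player character and damages it on contact.
; BeginPlay starts an AI MoveTo on the player, and both success and failure call the move event again as well as looping back after a delay.
; Capsule overlap with a Player-tagged actor starts a once-per-second damage loop that has no end-overlap or exit check.
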(event `self.ReceiveBeginPlay`
  (`self.movezombie`))

(event `movezombie`
  (`|AIMoveTo` self (0.0 0.0 0.0) (`GameplayStatics.GetPlayerCharacter` 0) 7.0 :!label _label
    (:`OnSuccess`
      (`self.movezombie`))
    (:`OnFail`
      (`self.movezombie`)))
  (`KismetSystemLibrary.Delay` 1.5)
  (goto _label))

(event `self.Capsule.OnComponentBeginOverlap`
  (params (OverlappedComponent :type "PrimitiveComponent Object Reference") (OtherActor :type "Actor Object Reference") (OtherComp :type "PrimitiveComponent Object Reference") (OtherBodyIndex :type Integer) (bFromSweep :type Boolean) (SweepResult :type "HitResult Structure (by ref)"))
  (if (`self.ActorHasTag` OtherActor "Player")
    (`GameplayStatics.ApplyDamage` OtherActor 10.0 null self :!label _label_2)
    (`KismetSystemLibrary.Delay` 1.0)
    (goto _label_2)))

(fn `UserConstructionScript`)